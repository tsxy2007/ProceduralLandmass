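; Actor that displays a procedurally generated noise texture on its Plane component.
; A shared function builds a noise map from size, scale, seed and fractal settings (octaves, persistence, lacunarity), then converts it to a texture.
; It feeds that texture into the Color parameter of a new dynamic instance of MTexture on the plane.
; This runs in both the Construction Script and BeginPlay, so the result also previews in the editor.
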(event `self.ReceiveBeginPlay`
  (`self.NewFunction`))

(fn `NewFunction`
  (bind _outnoisemap (`ProceduralLandmassBPLibrary.GenerateNoiseMap` (`self.Width`) (`self.Height`) (`self.Scale`) (`self.Octaves`) (`self.Persistance`) (`self.Lacunarity`) (`self.Seed`)))
  (bind _returnvalue (`ProceduralLandmassBPLibrary.GenerateNoiseTexture` (`self.Width`) (`self.Height`) _outnoisemap))
  (bind _returnvalue_2 (`KismetMaterialLibrary.CreateDynamicMaterialInstance` (`self.M_Texture`)))
  (`MaterialInstanceDynamic.SetTextureParameterValue` _returnvalue_2 "Color" _returnvalue)
  (`PrimitiveComponent.SetMaterial` (`self.Plane`) 0 _returnvalue_2))

(fn `UserConstructionScript`
  (`self.NewFunction`))