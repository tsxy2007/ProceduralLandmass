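; BP_ProcessLand_CS is an actor that previews procedurally generated, noise-based terrain as a color texture on a plane.
; Its Construction Script calls NoiseFunc, which runs ExecuteGPUNoiseMap with terrain types, chunk size, fractal noise settings, seed, offset and two render targets.
; It then feeds the color render target into a dynamic M_Color material applied to the Plane, with no runtime tick logic.
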(event `self.ReceiveTick`
  (params (DeltaSeconds :type "Float (single-precision)")))

(event `NoiseFunc`
  (`ProceduralLandmassNoiseCS_AsyncExecution.ExecuteGPUNoiseMap` (`self.In Terrain Types`) (`self.Chunk Size`) (`self.Scale`) (`self.Octaves`) (`self.Persistence`) (`self.Lacunarity`) (`self.Seed`) (`self.Offset`) (`self.RT`) (`self.Color RT`))
  (bind _returnvalue (`KismetMaterialLibrary.CreateDynamicMaterialInstance` "/ProceduralLandmass/UE53/M_Color.M_Color" "None"))
  (`MaterialInstanceDynamic.SetTextureParameterValue` _returnvalue "TerrainColorTexture" (`self.Color RT`))
  (`PrimitiveComponent.SetMaterial` (`self.Plane`) 0 _returnvalue))

(fn `NewFunction`)

(fn `UserConstructionScript`
  (`self.NoiseFunc`))