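; BP_Color is a procedural terrain preview actor that displays a generated noise map on its Plane component.
; NewFunction builds the noise map, then DrawMode selects a grayscale noise texture, a terrain-type color texture, or a height-curve mesh with that color texture.
; Each mode feeds its texture into a dynamic M_Color material on the Plane, and Mesh mode also replaces its static mesh.
; No live event or construction script calls NewFunction.
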(event `self.ReceiveBeginPlay`)

(fn `NewFunction`
  (bind _outnoisemap (`ProceduralLandmassBPLibrary.GenerateNoiseMap` (`self.Chunk Size`) (`self.Scale`) (`self.Octaves`) (`self.Persistance`) (`self.Lacunarity`) (`self.Seed`) (`self.Offset`)))
  (switch `ENoiseDrawMode` (`self.drawMode`)
    (:`ENDM_Noise`
      (bind _returnvalue (`ProceduralLandmassBPLibrary.GenerateNoiseTexture` (`self.Chunk Size`) _outnoisemap))
      (bind _returnvalue_2 (`KismetMaterialLibrary.CreateDynamicMaterialInstance` "/ProceduralLandmass/UE53/M_Color.M_Color" "None"))
      (`MaterialInstanceDynamic.SetTextureParameterValue` _returnvalue_2 "TerrainColorTexture" _returnvalue)
      (`PrimitiveComponent.SetMaterial` (`self.Plane`) 0 _returnvalue_2))
    (:`ENDM_Color`
      (bind _returnvalue_3 (`ProceduralLandmassBPLibrary.GenerateColorNoiseTexture` (`self.Chunk Size`) (`self.terrainTypes`) _outnoisemap))
      (bind _returnvalue_4 (`KismetMaterialLibrary.CreateDynamicMaterialInstance` "/ProceduralLandmass/UE53/M_Color.M_Color" "None"))
      (`MaterialInstanceDynamic.SetTextureParameterValue` _returnvalue_4 "TerrainColorTexture" _returnvalue_3)
      (`PrimitiveComponent.SetMaterial` (`self.Plane`) 0 _returnvalue_4))
    (:`ENDM_Mesh`
      (bind _returnvalue_5 (`ProceduralLandmassBPLibrary.GenerateTerrainMesh` (`self.Chunk Size`) (`self.Height Scale`) _outnoisemap (`self.Height Curve`) (`self.LODLevels`)))
      (bind _returnvalue_6 (`TerrainMeshData.CreateMesh` _returnvalue_5))
      (`StaticMeshComponent.SetStaticMesh` (`self.Plane`) _returnvalue_6)
      (bind _returnvalue_7 (`ProceduralLandmassBPLibrary.GenerateColorNoiseTexture` (`self.Chunk Size`) (`self.terrainTypes`) _outnoisemap))
      (bind _returnvalue_8 (`KismetMaterialLibrary.CreateDynamicMaterialInstance` "/ProceduralLandmass/UE53/M_Color.M_Color" "None"))
      (`MaterialInstanceDynamic.SetTextureParameterValue` _returnvalue_8 "TerrainColorTexture" _returnvalue_7)
      (`PrimitiveComponent.SetMaterial` (`self.Plane`) 0 _returnvalue_8))))

(fn `UserConstructionScript`)